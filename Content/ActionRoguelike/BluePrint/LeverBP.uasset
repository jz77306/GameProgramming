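; An interactable lever that grants the pawn using it a KeyCard gameplay tag.
; On Interact it snaps the handle mesh to a pitched-down rotation and adds the tag directly to the ActiveGameplayTags container on the instigator's SActionComponent.
; The interact text is empty, and a disconnected leftover branch that would explode a selected ExplosiveBarrel never runs.
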(event EventBeginPlay)

(event Collision|EventActorBeginOverlap
  (params (OtherActor :type Actor%20Object%20Reference)))

(event EventTick
  (params (DeltaSeconds :type Float%20%28single-precision%29)))

(event EventInteract
  (params (InstigatorPawn :type Pawn%20Object%20Reference))
  (Transformation|SetRelativeRotation (Variables|Default|GetHandleMesh) (Math|Rotator|MakeRotator 0.0 -3e+01 0.0) false false)
  (GameplayTags|AddGameplayTag (Variables|/Script/ActionRoguelike.SActionComponent|GetActiveGameplayTags (Actor|GetComponentbyClass InstigatorPawn "/Script/ActionRoguelike.SActionComponent")) (Variables|Default|GetKeyCard) :!class /Script/GameplayTags.BlueprintGameplayTagLibrary))

(fn ConstructionScript)

(fn GetInteractText
  (params (InstigatorPawn :type Pawn%20Object%20Reference))
  (return ""))