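; Player character Blueprint that layers input, UI and audio feedback onto the character's action and attribute components.
; The Parry input starts the projectile-reflecting Parry action by name through ActionComp.
; BeginPlay attaches a health widget above the character, and AttributeComp's health-change event plays attached hurt or death sounds.
; An unconnected test snippet would apply a Stunned debuff after a short delay.
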(event OnHealthChanged(AttributeComp)
  (params (InstigatorActor :type Actor%20Object%20Reference) (OwningComp :type S%20Attribute%20Component%20Object%20Reference) (NewValue :type Float%20%28single-precision%29) (Delta :type Float%20%28single-precision%29))
  (if (> NewValue 0.0) ; IsAlive
    (if (< Delta 0.0)
      (Audio|SpawnSoundAttached (Variables|Default|GetTakeDamageCue) (Variables|Transformation|GetRootComponent) "None" "0, 0, 0" "0, 0, 0" "KeepRelativeOffset" false 1.0 1.0 0.0 0 0))
    (else
      (Audio|SpawnSoundAttached (Variables|Default|GetDeathCue) (Variables|Transformation|GetRootComponent) "None" "0, 0, 0" "0, 0, 0" "KeepRelativeOffset" false 1.0 1.0 0.0 0 0))))

(event EventBeginPlay
  ;[1 1 1] Show Health Above player Characters
  (bind _returnvalue (UserInterface|CreateWidget "/Game/ActionRoguelike/UI/MinionHealth_Widget.MinionHealth_Widget_C" 0 self))
  (UserInterface|Viewport|AddtoViewport _returnvalue 0))

(event Input|ActionEvents|InputActionParry
  (params (Key :type Key%20Structure))
  ;[1 1 1] Activate 'Parry' Buff that reflects incoming projectiles.
  (:Pressed
    (Class|SActionComponent|StartActionbyName (Variables|Default|GetActionComp) self "Parry")))

(fn ConstructionScript)