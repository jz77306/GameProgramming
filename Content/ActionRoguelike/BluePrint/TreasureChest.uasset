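; TreasureChest is an interactable chest Blueprint whose Interact event calls the parent implementation, then prints a debug message.
; The remaining graph logic is disconnected and never runs.
; It holds a RequiredKeyCard gameplay tag check against SActionComponent, a FlipFlop timeline that pitches the lid open or closed with particles after opening, and a LidOpened debug print.
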(event EventTick
  (params (DeltaSeconds :type Float%20%28single-precision%29)))

(event EventInteract
  (params (InstigatorPawn :type Pawn%20Object%20Reference))
  (|CallParentFunction InstigatorPawn)
  (Development|PrintString "TreasureChest Interact (BP)" true true "(R=0.000000,G=0.310950,B=1.000000,A=1.000000)" 1e+01))

(fn ConstructionScript)